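; BP_Pickup is an interactable item actor that the player can pick up, apparently a key.
; On BeginPlay it caches the PBP_Topdown2D actor as its player reference.
; Its Interact function checks that the player's current inventory room is not at the maximum slot count, then prints a pickup message, destroys itself and returns a can-be-picked-up flag with its pickup name.
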(event EventBeginPlay
  (bind _returnvalue (Actor|GetActorOfClass "/Game/TopDownBP/Character/RPGCharacter/Blueprint/PBP_Topdown2D.PBP_Topdown2D_C"))
  (Variables|Default|SetPCReference _returnvalue))

(event Collision|EventActorBeginOverlap
  (params (OtherActor :type Actor%20Object%20Reference)))

(event EventTick
  (params (DeltaSeconds :type Float%20%28single-precision%29)))

(fn ConstructionScript)

(fn Interact
  (bind _pcreference (Variables|Default|GetPCReference))
  (if (not (== (Variables|/Game/TopDownBP/Character/RPGCharacter/Blueprint/PBP_Topdown2D.PBP_Topdown2D_C|GetMaxInventorySlots _pcreference) (Variables|/Game/TopDownBP/Character/RPGCharacter/Blueprint/PBP_Topdown2D.PBP_Topdown2D_C|GetCurrentInventoryRoom _pcreference)))
    (Development|PrintString "Picked up key")
    (Actor|DestroyActor)
    (return true (Variables|Default|GetNameOfPickup))))