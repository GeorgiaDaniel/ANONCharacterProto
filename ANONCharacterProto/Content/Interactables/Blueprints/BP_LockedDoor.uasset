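; BP_LockedDoor is an interactable locked door that the player opens by spending a key.
; BeginPlay caches the PBP_Topdown2D actor.
; Interact looks up "Key" in that actor's PlayerInventory; if found, it decrements the value, calls InventoryNumberIncorDec with -1 and destroys the door, otherwise it prints "Locked".
; The key check tests only whether the entry exists, not its count.
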(event EventBeginPlay
  (bind _returnvalue (Actor|GetActorOfClass "/Game/TopDownBP/Character/RPGCharacter/Blueprint/PBP_Topdown2D.PBP_Topdown2D_C"))
  (Variables|Default|SetPCReference _returnvalue))

(fn ConstructionScript)

(fn Interact
  (bind _pcreference (Variables|Default|GetPCReference))
  (bind _playerinventory (Variables|/Game/TopDownBP/Character/RPGCharacter/Blueprint/PBP_Topdown2D.PBP_Topdown2D_C|GetPlayerInventory _pcreference))
  (bind (_value _returnvalue) (Utilities|Map|Find _playerinventory "Key"))
  (if _returnvalue
    (Math|Integer|DecrementInt _value
      (:%20%20
        (Default|InventoryNumberIncorDec (Variables|Default|GetPCReference) -1)
        (Actor|DestroyActor)
        (return false "")))
    (else
      (Development|PrintString "Locked"))))